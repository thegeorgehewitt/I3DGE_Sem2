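; Checkpoint actor with a bobbing, spinning sprite that reports a new respawn point when the player first touches it.
; Box overlap by the player clears its active flag and broadcasts its transform through ECheckpointHit, then plays explosion particles, sound and a UI fade, hiding the sprite.
; SaveData and LoadData persist the active flag; older code writing SpawnTransform directly to the player and Game Instance is left unconnected.
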(event OnComponentBeginOverlap(Box)
  (params (OverlappedComponent :type Primitive%20Component%20Object%20Reference) (OtherActor :type Actor%20Object%20Reference) (OtherComp :type Primitive%20Component%20Object%20Reference) (OtherBodyIndex :type Integer) (bFromSweep :type Boolean) (SweepResult :type Hit%20Result%20Structure%20%28by%20ref%29))
  ;[1 1 1] Updates the player respawn position on touch - this is the only information that is pushed to Game Instance (so all puzzles will completely reset, for example)
  (bind _asplayer_character (Utilities|Casting|CastToPlayerCharacter OtherActor))
  (if (Variables|Default|GetCheckpointActive)
    (Variables|Default|SetCheckpointActive false)
    (Default|CallECheckpointHit (Transformation|GetActorTransform))
    (CallFunction|CloseCheckpoint)))

(event Custom|CloseCheckpoint
  ;[1 1 1] Updates the player respawn position on touch - this is the only information that is pushed to Game Instance (so all puzzles will completely reset, for example)
  (Class|NiagaraComponent|SetAsset (Variables|Default|GetCheckpointParticles) "/Game/Core/Particles/Niagara/PS_CheckpointExplode.PS_CheckpointExplode" true)
  (Rendering|SetVisibility (Variables|Default|GetPaperSprite) false false)
  (UserInterface|Animation|PlayAnimation (Variables|/Game/Framework/Blueprints/PlayerCharacter.PlayerCharacter_C|GetMyUI (stale OnComponentBeginOverlap(Box) _asplayer_character)) (Variables|/Game/Core/UI/PlayerHud.PlayerHud_C|GetCheckpointFade (Variables|/Game/Framework/Blueprints/PlayerCharacter.PlayerCharacter_C|GetMyUI (stale OnComponentBeginOverlap(Box) _asplayer_character))) 0.0 1 "Forward" 1.0 false)
  (Audio|PlaySoundatLocation "/Game/Core/Audio/switch_007_Cue.switch_007_Cue" (Transformation|GetActorLocation) "0, 0, 0" 1.0 1.0 0.0 0 0 0 0))

(event EventBeginPlay
  (bind _papersprite (Variables|Default|GetPaperSprite))
  ;[1 1 1] Updates the player respawn position on touch - this is the only information that is pushed to Game Instance (so all puzzles will completely reset, for example)
  (bind _output_get (Variables|Default|SetSpriteStartLoc (Transformation|GetWorldLocation (Variables|Default|GetPaperSprite))))
  (bind _newtrack_1 (Timeline|Sprite%20Bob Play)
    (:Update
      (Transformation|SetWorldLocation _papersprite (Math|Vector|Lerp(Vector) _output_get (+ _output_get "0, 0,50.000000") _newtrack_1) false false)
      (Transformation|AddLocalRotation _papersprite "0,1.000000, 0" false false))))

(event EventLoadData
  (params (ActorState :type Boolean) (ActorData :type Transform))
  (bind _output_get (Variables|Default|SetCheckpointActive ActorState))
  (if _output_get
    (Class|NiagaraComponent|SetRenderingEnabled (Variables|Default|GetCheckpointParticles) false)))

(fn ConstructionScript)

(fn SaveData
  (return (Variables|Default|GetCheckpointActive) (Transformation|GetActorTransform)))