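; Actor component that respawns its owner at its starting location when destroyed, intended for prerequisite puzzle objects and included on Pick Up Object by default.
; BeginPlay caches the owner's transform.
; On EndPlay, if RespawnIfDestroyed is set, it spawns a RespawnHelper actor carrying the owner's class and start transform, handing off the respawn to an actor that outlives the component.
; The handoff carries only class and transform, without other instance state.
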(event Custom|Pass%20Details%20to%20Respawn%20Helper
  ;[1 1 1] Add this component to any actor that you wish to respawn when destroyed, and tick the Respawn if Destroyed boolean. When destroyed (either by the player or by it falling out the world, or whatever) an exact copy of the object will be respawned at its starting location. Use this on any puzzle objects that are pre-requisites. Present in the Pick Up Object by default.
  (Game|SpawnActorfromClass "/Game/Core/Blueprints/RespawnHelper.RespawnHelper_C" (Math|Transform|MakeTransform "0, 0, 0" "0, 0, 0" "1,1,1") "AlwaysSpawn" 0 (Utilities|Struct|MakeRespawnItemInfo (Utilities|GetClass (Components|GetOwner)) (Variables|Default|GetStartTransform) (Variables|Default|GetRespawn%20if%20Destroyed?)) 0))

(event EventBeginPlay
  ;[1 1 1] Add this component to any actor that you wish to respawn when destroyed, and tick the Respawn if Destroyed boolean. When destroyed (either by the player or by it falling out the world, or whatever) an exact copy of the object will be respawned at its starting location. Use this on any puzzle objects that are pre-requisites. Present in the Pick Up Object by default.
  (Variables|Default|SetStartTransform (Transformation|GetActorTransform (Components|GetOwner))))

(event EventEndPlay
  (params (EndPlayReason :type EEndPlayReason%20Enum :default "Destroyed"))
  ;[1 1 1] Add this component to any actor that you wish to respawn when destroyed, and tick the Respawn if Destroyed boolean. When destroyed (either by the player or by it falling out the world, or whatever) an exact copy of the object will be respawned at its starting location. Use this on any puzzle objects that are pre-requisites. Present in the Pick Up Object by default.
  (if (Variables|Default|GetRespawn%20if%20Destroyed?)
    (CallFunction|PassDetailstoRespawnHelper)))