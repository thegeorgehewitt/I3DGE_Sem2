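; Game mode for the goblin game, handling the main menu, player spawning and checkpoint respawns.
; BeginPlay forces windowed resolution, binds checkpoints, then shows the menu or a timed loading widget over a cine-camera view.
; Checkpoint hits snapshot SaveInterface actors into a map, plus respawn transform and weapon classes.
; Restarting restores those actors in place without reloading, then respawns the player at the checkpoint, falling back to PlayerStart.
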(event Custom|Click%20Start
  (bind _mainmenu (Variables|Default|GetMainMenu))
  (bind _fadeanim (Variables|/Game/Core/UI/MainMenu.MainMenu_C|GetFadeAnim _mainmenu))
  ;[1 1 1] Main Menu Commands
  (UserInterface|Animation|PlayAnimation _mainmenu _fadeanim 0.0 1 "Reverse" 2.0 false)
  (Class|UserWidget|BindtoAnimationFinished (Variables|Default|GetMainMenu) _fadeanim (delegate Custom|Begin%20Game)))

(event Custom|Begin%20Game%20After%20Load
  ;[1 1 1] OpenGame
  (CallFunction|BeginGame)
  (Widget|RemovefromParent (Variables|Default|GetLoadingWidget)))

(event Custom|Begin%20Game
  (bind _returnvalue (Game|GetPlayerController 0))
  (bind _respawntransform (Variables|Default|GetRespawnTransform))
  (bind _mainmenu (Variables|Default|GetMainMenu))
  ;[1 1 1] Main Menu Commands
  ;[1 1 1] Start Game
  (Utilities|IsValid _mainmenu
    (:Is%20Valid
      (Widget|RemovefromParent _mainmenu))
    (:Is%20Not%20Valid
      _))
  (Variables|/Script/Engine.PlayerController|SetbShowMouseCursor _returnvalue false)
  (Input|SetInputModeGameOnly _returnvalue)
  (Utilities|FlowControl|Sequence
    (:then_0
      (if (Variables|Default|GetUseCheckpoint)
        (CallFunction|SpawnPlayer (Math|Transform|MakeTransform (.location _respawntransform) (.rotation _respawntransform) "1.000000,1.000000,1.000000"))
        (else
          (bind _outactors (Actor|GetAllActorsOfClass "/Script/Engine.PlayerStart"))
          (CallFunction|SpawnPlayer (Math|Transform|MakeTransform (.location (Transformation|GetActorTransform (Utilities|Array|Get(acopy) _outactors))) (.rotation (Transformation|GetActorTransform (Utilities|Array|Get(acopy) _outactors))) "1.000000,1.000000,1.000000")))))
    (:then_1
      (Variables|/Game/Core/Blueprints/GoblinGameInstance.GoblinGameInstance_C|SetToMainMenu? (Variables|Default|GetGameInstance) false))))

(event Custom|Quit%20Event
  ;[1 1 1] Main Menu Commands
  (Game|QuitGame 0 "Quit" false))

(event Custom|RestartLevel
  (params (DestroyedActor :type Actor%20Object%20Reference))
  (bind _outactors (Actor|GetAllActorswithInterface "/Game/Core/Blueprints/Interfaces/SaveInterface.SaveInterface_C"))
  (for _array_element _outactors
    (if (.ReturnValue (Utilities|Map|Find (Variables|Default|GetSavedActors) _array_element))
      (Class|SaveInterface|LoadData(Message) _array_element (.ActorState (Utilities|Struct|BreakS_ActorSaveData (.Value (Utilities|Map|Find (Variables|Default|GetSavedActors) _array_element)))) (.ActorData (Utilities|Struct|BreakS_ActorSaveData (.Value (Utilities|Map|Find (Variables|Default|GetSavedActors) _array_element)))))))
  ;[1 1 1] Load Settings
  (bind _outactors_2 (Actor|GetAllActorsOfClass "/Script/CinematicCamera.CineCameraActor"))
  (Game|Player|SetViewTargetwithBlend (Game|GetPlayerController 0) (Utilities|Array|Get(acopy) _outactors_2) 0.0 "VTBlend_Linear" 0.0 false)
  (if (Variables|/Game/Core/Blueprints/GoblinGameInstance.GoblinGameInstance_C|GetToMainMenu? (Variables|Default|GetGameInstance))
    ;[1 1 1] Open Main Menu
    (Utilities|FlowControl|Sequence
      (:then_0
        (Variables|/Script/Engine.PlayerController|SetbShowMouseCursor (Game|GetPlayerController 0) true))
      (:then_1
        (bind _returnvalue (UserInterface|CreateWidget "/Game/Core/UI/MainMenu.MainMenu_C"))
        (bind _output_get (Variables|Default|SetMainMenu _returnvalue))
        (UserInterface|Viewport|AddtoViewport _output_get 0)
        (Variables|/Game/Core/UI/MainMenu.MainMenu_C|SetMyOwner _output_get self)
        (Input|SetInputModeUIOnly (Game|GetPlayerController 0) (Variables|Default|GetMainMenu) "DoNotLock")))
    (else
      ;[1 1 1] OpenGame
      (bind _returnvalue_2 (UserInterface|CreateWidget "/Game/Core/UI/LoadingWidget.LoadingWidget_C"))
      (bind _output_get_2 (Variables|Default|SetLoadingWidget _returnvalue_2))
      (UserInterface|Viewport|AddtoViewport _output_get_2 0)
      (Utilities|Time|SetTimerbyEvent (delegate Custom|Begin%20Game%20After%20Load) 1.3))))

(event Custom|CheckpointHit
  (params (CheckpointTransform :type Transform))
  (bind _playercharacter (Variables|Default|GetPlayerCharacter))
  (bind _weaponmanager (Variables|/Game/Framework/Blueprints/PlayerCharacter.PlayerCharacter_C|GetWeaponManager _playercharacter))
  (Variables|Default|SetRespawnTransform CheckpointTransform)
  (Variables|Default|SetUseCheckpoint true)
  (Utilities|Map|Clear (Variables|Default|GetSavedActors))
  (bind _outactors (Actor|GetAllActorswithInterface "/Game/Core/Blueprints/Interfaces/SaveInterface.SaveInterface_C"))
  (for _array_element _outactors
    (bind (_actorstate _actordata) (Class|SaveInterface|SaveData(Message) _array_element))
    (Utilities|Map|Add (Variables|Default|GetSavedActors) _array_element (Utilities|Struct|MakeS_ActorSaveData _actorstate _actordata)))
  (Utilities|Struct|SetmembersinS_PlayerSaveData (Variables|Default|GetPlayerCheckpointData) (Utilities|GetClass (Variables|/Game/Core/Blueprints/Components/BP_WeaponManager.BP_WeaponManager_C|GetMeleeWeapon _weaponmanager)) (Utilities|GetClass (Variables|/Game/Core/Blueprints/Components/BP_WeaponManager.BP_WeaponManager_C|GetRangedWeapon _weaponmanager))))

(event Custom|SpawnPlayer
  (params (SpawnTransform :type Transform))
  (bind _playercheckpointdata (Variables|Default|GetPlayerCheckpointData))
  (bind _returnvalue (Game|SpawnActorfromClass "/Game/Framework/Blueprints/PlayerCharacter.PlayerCharacter_C" SpawnTransform "Undefined" 0 0))
  (bind _output_get (Variables|Default|SetPlayerCharacter _returnvalue))
  (Pawn|Possess (Game|GetPlayerController 0) _output_get)
  (Game|BindEventtoOnDestroyed (Variables|Default|GetPlayerCharacter) (EventDispatchers|CreateEvent :!event Custom|RestartLevel))
  (if (and (Utilities|IsValidClass (.meleeweapon _playercheckpointdata)) (Utilities|IsValidClass (.rangedweapon _playercheckpointdata)))
    (Variables|/Game/Core/Blueprints/Components/BP_WeaponManager.BP_WeaponManager_C|SetDefaultMeleeWeapon (Variables|/Game/Framework/Blueprints/PlayerCharacter.PlayerCharacter_C|GetWeaponManager (Variables|Default|GetPlayerCharacter)) (.meleeweapon _playercheckpointdata))
    (Variables|/Game/Core/Blueprints/Components/BP_WeaponManager.BP_WeaponManager_C|SetDefaultRangedWeapon (Variables|/Game/Framework/Blueprints/PlayerCharacter.PlayerCharacter_C|GetWeaponManager (Variables|Default|GetPlayerCharacter)) (.rangedweapon _playercheckpointdata)))
  (Default|Init (Variables|Default|GetPlayerCharacter)))

(event EventBeginPlay
  (bind _returnvalue (Settings|GetGameUserSettings))
  (Class|GameUserSettings|SetFullscreenMode _returnvalue "Windowed")
  (Class|GameUserSettings|SetScreenResolution _returnvalue (Utilities|Struct|MakeIntPoint 1280 720))
  ;[1 1 1] Load Settings
  (Class|GameUserSettings|ApplySettings _returnvalue false)
  (bind _asgoblin_game_instance (Utilities|Casting|CastToGoblinGameInstance (Game|GetGameInstance)))
  (Variables|Default|SetGameInstance _asgoblin_game_instance)
  (bind _outactors (Actor|GetAllActorsOfClass "/Game/Framework/Blueprints/CheckPoint.CheckPoint_C"))
  (for _array_element _outactors
    (EventDispatchers|BindEventtoECheckpointHit _array_element (EventDispatchers|CreateEvent :!event Custom|CheckpointHit)))
  (bind _outactors_2 (Actor|GetAllActorsOfClass "/Script/CinematicCamera.CineCameraActor"))
  (Game|Player|SetViewTargetwithBlend (Game|GetPlayerController 0) (Utilities|Array|Get(acopy) _outactors_2) 0.0 "VTBlend_Linear" 0.0 false)
  (if (Variables|/Game/Core/Blueprints/GoblinGameInstance.GoblinGameInstance_C|GetToMainMenu? (Variables|Default|GetGameInstance))
    ;[1 1 1] Open Main Menu
    (Utilities|FlowControl|Sequence
      (:then_0
        (Variables|/Script/Engine.PlayerController|SetbShowMouseCursor (Game|GetPlayerController 0) true))
      (:then_1
        (bind _returnvalue_2 (UserInterface|CreateWidget "/Game/Core/UI/MainMenu.MainMenu_C"))
        (bind _output_get (Variables|Default|SetMainMenu _returnvalue_2))
        (UserInterface|Viewport|AddtoViewport _output_get 0)
        (Variables|/Game/Core/UI/MainMenu.MainMenu_C|SetMyOwner _output_get self)
        (Input|SetInputModeUIOnly (Game|GetPlayerController 0) (Variables|Default|GetMainMenu) "DoNotLock")))
    (else
      ;[1 1 1] OpenGame
      (bind _returnvalue_3 (UserInterface|CreateWidget "/Game/Core/UI/LoadingWidget.LoadingWidget_C"))
      (bind _output_get_2 (Variables|Default|SetLoadingWidget _returnvalue_3))
      (UserInterface|Viewport|AddtoViewport _output_get_2 0)
      (Utilities|Time|SetTimerbyEvent (delegate Custom|Begin%20Game%20After%20Load) 1.3))))

(fn ConstructionScript)