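; Character component that manages one melee and one ranged weapon slot, spawning defaults on init and dropping the old weapon when replaced.
; Weapons attach to hand or hip/back sockets chosen by weapon and equip type.
; Draw and holster use the weapon's draw montage, played in reverse for holstering, with notifies timing the reattachment.
; Switching while drawn holsters first, then swaps and redraws; a held attack button fires after drawing.
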(event Custom|AddWeapon
  (params (WeaponToAdd :type Weapon%20Object%20Reference))
  (Utilities|FlowControl|Sequence
    (:then_0
      (Default|InitWeapon WeaponToAdd (Variables|Default|GetOwning%20Character)))
    (:then_1
      (switch Utilities|FlowControl|Switch|SwitchonWeaponTypes (Variables|/Game/Core/Blueprints/Weapons/Weapon.Weapon_C|GetWeaponType WeaponToAdd)
        (:NewEnumerator0
          (bind _meleeweapon (Variables|Default|GetMeleeWeapon)
            (:then
              (CallFunction|DropWeapon _meleeweapon))
            (:else
              _))
          (bind _asweapon_melee (Utilities|Casting|CastToWeapon_Melee WeaponToAdd))
          (bind _output_get (Variables|Default|SetMeleeWeapon _asweapon_melee))
          (Transformation|AttachComponentToComponent _output_get (Variables|/Script/Engine.Character|GetMesh (Variables|Default|GetOwning%20Character)) (Utilities|Select :Index (Variables|/Game/Core/Blueprints/Weapons/Weapon.Weapon_C|GetEquipType _output_get) :NewEnumerator0 (Variables|Default|GetLeftHipWeapon) :NewEnumerator1 (Variables|Default|GetLeftBackWeapon) :NewEnumerator2 "None") "SnapToTarget" "SnapToTarget" "KeepWorld" true)
          (bind _currentweapon (Variables|Default|GetCurrentWeapon)
            (:then
              (if (Utilities|Enum|Equal(Enum) (Variables|/Game/Core/Blueprints/Weapons/Weapon.Weapon_C|GetWeaponType _currentweapon) "NewEnumerator0")
                (Variables|Default|SetCurrentWeapon (Variables|Default|GetMeleeWeapon))
                (if (Variables|Default|GetWeaponDrawn) :!label _label
                  (CallFunction|AttachWeapon))))
            (:else)))
        (:NewEnumerator1
          (bind _rangedweapon (Variables|Default|GetRangedWeapon)
            (:then
              (CallFunction|DropWeapon _rangedweapon))
            (:else
              _))
          (bind _asweapon_ranged (Utilities|Casting|CastToWeapon_Ranged WeaponToAdd))
          (bind _output_get_2 (Variables|Default|SetRangedWeapon _asweapon_ranged))
          (Transformation|AttachComponentToComponent _output_get_2 (Variables|/Script/Engine.Character|GetMesh (Variables|Default|GetOwning%20Character)) (Utilities|Select :Index (Variables|/Game/Core/Blueprints/Weapons/Weapon.Weapon_C|GetEquipType _output_get_2) :NewEnumerator0 (Variables|Default|GetRightHipWeapon) :NewEnumerator1 (Variables|Default|GetRightBackWeapon) :NewEnumerator2 "None") "SnapToTarget" "SnapToTarget" "KeepWorld" true)
          (bind _currentweapon_2 (Variables|Default|GetCurrentWeapon)
            (:then
              (if (Utilities|Enum|Equal(Enum) (Variables|/Game/Core/Blueprints/Weapons/Weapon.Weapon_C|GetWeaponType _currentweapon_2) "NewEnumerator1")
                (Variables|Default|SetCurrentWeapon (Variables|Default|GetRangedWeapon))
                (goto _label)))
            (:else)))))))

(event Custom|DropWeapon
  (params (WeaponToDrop :type Weapon%20Object%20Reference))
  (bind _owning_character (Variables|Default|GetOwning%20Character))
  (Transformation|DetachFromActor WeaponToDrop "KeepWorld" "KeepWorld" "KeepWorld")
  (Transformation|SetActorLocation WeaponToDrop (+ (Transformation|GetActorLocation _owning_character) (* (Transformation|GetActorForwardVector _owning_character) 2e+01)) false false)
  (Default|DropWeapon WeaponToDrop))

(event Custom|PostHolsterSwitch
  (if (== (Variables|Default|GetCurrentWeapon) (Variables|Default|GetMeleeWeapon))
    (Variables|Default|SetCurrentWeapon (Variables|Default|GetRangedWeapon))
    (else
      (Variables|Default|SetCurrentWeapon (Variables|Default|GetMeleeWeapon))))
  (if (Variables|Default|GetWeaponDrawn)
    (CallFunction|DrawWeapon)))

(event Custom|AttachWeapon
  (bind _currentweapon (Variables|Default|GetCurrentWeapon))
  (Transformation|AttachComponentToComponent _currentweapon (Variables|/Script/Engine.Character|GetMesh (Variables|Default|GetOwning%20Character)) (Utilities|Select :Index (Variables|/Game/Core/Blueprints/Weapons/Weapon.Weapon_C|GetWeaponType _currentweapon) :NewEnumerator0 (Variables|Default|GetMeleeHoldSocket) :NewEnumerator1 (Variables|Default|GetRangedHoldSocket)) "SnapToTarget" "SnapToTarget" "KeepWorld" true))

(event Custom|HolsterWeapon
  (params (Switching :type Boolean))
  (bind _currentweapon (Variables|Default|GetCurrentWeapon))
  (bind _currentweapon_2 (Variables|Default|GetCurrentWeapon))
  (bind _equiptype (Variables|/Game/Core/Blueprints/Weapons/Weapon.Weapon_C|GetEquipType _currentweapon_2))
  (bind _weapondrawanim (Variables|/Game/Core/Blueprints/Weapons/Weapon.Weapon_C|GetWeaponDrawAnim _currentweapon))
  (if (Variables|Default|GetWeaponDrawn)
    (Animation|Montage|PlayMontage (Variables|/Script/Engine.Character|GetMesh (Variables|Default|GetOwning%20Character)) _weapondrawanim (* (Variables|/Game/Core/Blueprints/Weapons/Weapon.Weapon_C|GetWeaponDrawSpeed _currentweapon) -1.0) (Variables|/Script/Engine.AnimSequenceBase|GetSequenceLength _weapondrawanim)
      (:then
        (if (not Switching)
          (Variables|Default|SetWeaponDrawn false)))
      (:OnNotifyBegin
        (Transformation|AttachComponentToComponent (Variables|Default|GetCurrentWeapon) (Variables|/Script/Engine.Character|GetMesh (Variables|Default|GetOwning%20Character)) (Utilities|Select :Index (Variables|/Game/Core/Blueprints/Weapons/Weapon.Weapon_C|GetWeaponType _currentweapon_2) :NewEnumerator0 (Utilities|Select :Index _equiptype :NewEnumerator0 (Variables|Default|GetLeftHipWeapon) :NewEnumerator1 (Variables|Default|GetLeftBackWeapon) :NewEnumerator2 "None") :NewEnumerator1 (Utilities|Select :Index _equiptype :NewEnumerator0 (Variables|Default|GetRightHipWeapon) :NewEnumerator1 (Variables|Default|GetRightBackWeapon) :NewEnumerator2 "None")) "SnapToTarget" "SnapToTarget" "KeepWorld" true)
        (if Switching
          (CallFunction|PostHolsterSwitch))))))

(event Custom|Init
  (params (OwningCharacter :type Player%20Character%20Object%20Reference))
  (Variables|Default|SetOwning%20Character OwningCharacter)
  (CallFunction|CreateDefaultWeapons))

(event Custom|CreateDefaultWeapons
  (Utilities|FlowControl|Sequence
    (:then_0
      (bind _returnvalue (Game|SpawnActorfromClass (Variables|Default|GetDefaultMeleeWeapon) (Math|Transform|MakeTransform "0, 0, 0" "0, 0, 0" "1.000000,1.000000,1.000000") "Undefined" 0 0))
      (CallFunction|AddWeapon _returnvalue))
    (:then_1
      (bind _returnvalue_2 (Game|SpawnActorfromClass (Variables|Default|GetDefaultRangedWeapon) (Math|Transform|MakeTransform "0, 0, 0" "0, 0, 0" "1.000000,1.000000,1.000000") "Undefined" 0 0))
      (CallFunction|AddWeapon _returnvalue_2))
    (:then_2
      (Variables|Default|SetCurrentWeapon (Variables|Default|GetMeleeWeapon)))))

(event Custom|DrawWeapon
  (bind _currentweapon (Variables|Default|GetCurrentWeapon))
  (if (not (Utilities|Enum|Equal(Enum) (Variables|/Game/Framework/Blueprints/PlayerCharacter.PlayerCharacter_C|GetMyState (Variables|Default|GetOwning%20Character)) "NewEnumerator1"))
    (Animation|Montage|PlayMontage (Variables|/Script/Engine.Character|GetMesh (Variables|Default|GetOwning%20Character)) (Variables|/Game/Core/Blueprints/Weapons/Weapon.Weapon_C|GetWeaponDrawAnim _currentweapon) (Variables|/Game/Core/Blueprints/Weapons/Weapon.Weapon_C|GetWeaponDrawSpeed _currentweapon)
      (:OnBlendOut
        (Variables|Default|SetWeaponDrawn true)
        (if (Variables|/Game/Framework/Blueprints/PlayerCharacter.PlayerCharacter_C|GetAttack%20Button%20Down (Variables|Default|GetOwning%20Character))
          (Default|Attack (Variables|Default|GetCurrentWeapon))))
      (:OnNotifyBegin
        (CallFunction|AttachWeapon)))))

(event Custom|SwitchWeapon
  (if (Variables|Default|GetWeaponDrawn)
    (CallFunction|HolsterWeapon true)
    (else
      (if (== (Variables|Default|GetCurrentWeapon) (Variables|Default|GetMeleeWeapon))
        (Variables|Default|SetCurrentWeapon (Variables|Default|GetRangedWeapon))
        (else
          (Variables|Default|SetCurrentWeapon (Variables|Default|GetMeleeWeapon))))
      (if (Variables|Default|GetWeaponDrawn)
        (CallFunction|DrawWeapon)))))