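; Base physics object the player picks up, carries and drops, with health, point damage, impact effects and transform save/load.
; Interact attaches it to the player's HoldingSocket with physics off; Drop detaches it and re-enables physics.
; Drops not in front overlap pawns until a pawn's overlap ends, avoiding collision.
; Preview mode makes it an overlap-only ghost with dynamic materials recoloured for placeable or blocked placement.
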(event OnComponentEndOverlap(StaticMesh)
  (params (OverlappedComponent :type Primitive%20Component%20Object%20Reference) (OtherActor :type Actor%20Object%20Reference) (OtherComp :type Primitive%20Component%20Object%20Reference) (OtherBodyIndex :type Integer))
  (if (not (Variables|Default|GetPreviewObject))
    (Utilities|Casting|CastToPawn OtherActor)
    (Collision|SetCollisionResponsetoChannel (Variables|Default|GetStaticMesh) "ECC_Pawn" "ECR_Block")))

(event Custom|ActivateObject)

(event Custom|SetPreview
  (bind _staticmesh (Variables|Default|GetStaticMesh))
  (Physics|SetSimulatePhysics _staticmesh false)
  (Collision|SetCollisionEnabled _staticmesh "QueryOnly")
  (Collision|SetCollisionProfileName _staticmesh "OverlapAll" true :!class /Script/Engine.PrimitiveComponent)
  (Variables|Default|SetDestroyedParticle 0)
  (Variables|/Game/Framework/Blueprints/RespawnComponent.RespawnComponent_C|SetRespawn%20if%20Destroyed? (Variables|Default|GetRespawnComponent) false)
  (for _array_element (Actor|GetComponentsByClass "/Script/Engine.StaticMeshComponent")
    (for _index (range 0 (- (Rendering|Material|GetNumMaterials _array_element) 1))
      (bind _returnvalue (Rendering|Material|CreateDynamicMaterialInstance _array_element _index "/Game/Core/Materials/MI_HeldPreview.MI_HeldPreview" "None" :!class /Script/Engine.PrimitiveComponent))
      (Utilities|Array|Add (Variables|Default|GetPreviewMaterials) _returnvalue))))

(event Custom|Death
  ;[1 1 1] Damage & Death
  (Niagara|SpawnSystematLocation "/Game/Core/Particles/Niagara/PS_Explode.PS_Explode" (Transformation|GetActorLocation))
  (Actor|DestroyActor))

(event Custom|Overlapping
  (for _array_element (Variables|Default|GetPreviewMaterials)
    (Rendering|Material|SetVectorParameterValue _array_element "PreviewColour" (Variables|Default|GetUnplaceableColour) :!class /Script/Engine.MaterialInstanceDynamic))
  (Variables|Default|SetOverlapped true))

(event Custom|ClearOverlap
  (for _array_element (Variables|Default|GetPreviewMaterials)
    (Rendering|Material|SetVectorParameterValue _array_element "PreviewColour" (Variables|Default|GetPlaceableColour) :!class /Script/Engine.MaterialInstanceDynamic))
  (Variables|Default|SetOverlapped false))

(event Collision|EventHit
  (params (MyComp :type Primitive%20Component%20Object%20Reference) (Other :type Actor%20Object%20Reference) (OtherComp :type Primitive%20Component%20Object%20Reference) (bSelfMoved :type Boolean) (HitLocation :type Vector :default "0, 0, 0") (HitNormal :type Vector :default "0, 0, 0") (NormalImpulse :type Vector :default "0, 0, 0") (Hit :type Hit%20Result%20Structure%20%28by%20ref%29))
  (bind _returnvalue (Math|Vector|VectorLength NormalImpulse))
  (if bSelfMoved
    (if (> _returnvalue 8e+05)
      (Audio|PlaySoundatLocation (Variables|Default|GetHitSound) HitLocation "0, 0, 0" (Math|Float|MapRangeClamped _returnvalue 1e+01 5e+02 0.0 1.0) 1.0 0.0 0 0 0 0)
      (Niagara|SpawnSystematLocation "/Game/Core/Particles/Niagara/PS_WallHit02.PS_WallHit02" HitLocation (Math|Conversions|RotationFromXVector HitNormal)))))

(event EventDestroyed
  (Niagara|SpawnSystematLocation (Variables|Default|GetDestroyedParticle) (Transformation|GetActorLocation)))

(event Game|Damage|EventPointDamage
  (params (Damage :type Float%20%28single-precision%29) (DamageType :type Damage%20Type%20Object%20Reference) (HitLocation :type Vector :default "0, 0, 0") (HitNormal :type Vector :default "0, 0, 0") (HitComponent :type Primitive%20Component%20Object%20Reference) (BoneName :type Name :default "None") (ShotFromDirection :type Vector :default "0, 0, 0") (InstigatedBy :type Controller%20Object%20Reference) (DamageCauser :type Actor%20Object%20Reference) (HitInfo :type Hit%20Result%20Structure%20%28by%20ref%29))
  ;[1 1 1] Damage & Death
  (if (Variables|Default|GetCanBeDamaged)
    (bind _output_get (Variables|Default|SetHealth (- (Variables|Default|GetHealth) Damage)))
    (if (<= _output_get 0.0)
      (CallFunction|Death)
      (else
        (Niagara|SpawnSystematLocation "/Game/Core/Particles/Niagara/PS_EnergyHit.PS_EnergyHit" HitLocation)))))

(event EventBeginPlay
  (Variables|Default|SetDefaultSpawnTransform (Transformation|GetActorTransform)))

(event EventDrop
  (params (Player :type Player%20Character%20Object%20Reference) (In%20Front? :type Boolean))
  (bind _staticmesh (Variables|Default|GetStaticMesh))
  ;[1 1 1] When dropped, detach, re-enable physics etc
  (Transformation|DetachFromActor "KeepWorld" "KeepWorld" "KeepWorld")
  (Physics|SetSimulatePhysics (Variables|Default|GetStaticMesh) true)
  (Collision|SetCollisionEnabled _staticmesh "QueryAndPhysics")
  (Utilities|FlowControl|Sequence
    (:then_0
      (if (not In%20Front?)
        (Collision|SetCollisionResponsetoChannel _staticmesh "ECC_Pawn" "ECR_Overlap")))
    (:then_1
      (EventDispatchers|UnbindallEventsfromOnDestroyed)
      (Utilities|IsValid Player
        (:Is%20Valid
          (Collision|IgnoreActorwhenMoving (Variables|Default|GetStaticMesh) Player false))))))

(event EventLoadData
  (params (ActorState :type Boolean) (ActorData :type Transform))
  (Transformation|SetActorTransform ActorData))

(fn ConstructionScript)

(fn Interact
  (params (Player :type Player%20Character%20Object%20Reference))
  (bind _staticmesh (Variables|Default|GetStaticMesh))
  ;[1 1 1] On pick up, attach to player
  (Transformation|AttachComponentToComponent (Variables|/Script/Engine.Character|GetMesh Player) "HoldingSocket" "SnapToTarget" "SnapToTarget" "KeepWorld" true)
  (Utilities|IsValid self
    (:Is%20Valid
      (Collision|IgnoreActorwhenMoving _staticmesh Player true)
      (Physics|SetSimulatePhysics _staticmesh false)
      (Collision|SetCollisionEnabled (Variables|Default|GetStaticMesh) "QueryOnly")
      (return))))

(fn SaveData
  (return false (Transformation|GetActorTransform)))