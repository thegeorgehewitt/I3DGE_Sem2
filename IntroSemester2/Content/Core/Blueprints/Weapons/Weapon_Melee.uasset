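; Melee weapon Blueprint that lunges the owning character forward and damages what it hits on an attack.
; AttackEffect starts a timeline-driven, swept lunge with foot dust, sphere-traces at a point ahead of the owner and shakes the camera.
; Each hit gets point damage, a forward-and-up impulse on simulating bodies, impact VFX and sound, using a pickup's own sound when available.
; HitEffect is an empty per-hit event.
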(event Custom|MeleeLunge
  (bind _owningcharacter (Variables|Default|GetOwningCharacter))
  (Niagara|SpawnSystematLocation "/Game/Core/Particles/Niagara/PS_Dust01.PS_Dust01" (Transformation|GetSocketLocation (Variables|/Script/Engine.Character|GetMesh (Variables|Default|GetOwningCharacter)) "LeftToeBase"))
  (Components|Timeline|SetPlayRate (Variables|Default|GetT_Lunge) (Variables|Default|GetLungeSpeed))
  (Variables|Default|SetLungeStartLocation (Transformation|GetActorLocation _owningcharacter))
  (bind _alpha (Timeline|T_Lunge PlayFromStart)
    (:Update
      (Transformation|SetActorLocation (Variables|Default|GetOwningCharacter) (Math|Vector|Lerp(Vector) (Variables|Default|GetLungeStartLocation) (+ (Variables|Default|GetLungeStartLocation) (* (Transformation|GetActorForwardVector _owningcharacter) (Variables|Default|GetLungeDistance))) _alpha) true false))))

(event Custom|HitEffect
  (params (AttackHit :type Hit%20Result%20Structure)))

(event EventAttackEffect
  (bind _returnvalue (CallFunction|GetAttackOrigin))
  (CallFunction|MeleeLunge)
  (bind _outhits (Collision|MultiSphereTraceForObjects _returnvalue _returnvalue (Variables|Default|GetWeaponRadius) (Utilities|Array|MakeArray "ObjectTypeQuery1" "ObjectTypeQuery2" "ObjectTypeQuery4") false 0 "None"))
  (for _array_element _outhits
    (CallFunction|ApplyDamage _array_element))
  (CameraShakes|StartCameraShake (Game|GetPlayerCameraManager 0) "/Game/Core/CameraShakes/GrabCameraShake.GrabCameraShake_C" (Variables|Default|GetCameraShakeScale) "CameraLocal" "0, 0, 0"))

(fn ConstructionScript
  (|CallParentFunction))

(fn ApplyDamage
  (params (HitResult :type Hit%20Result%20Structure))
  (bind (_bblockinghit _binitialoverlap _time _distance _location _impactpoint _normal _impactnormal _physmat _hitactor) (Collision|BreakHitResult HitResult))
  (bind _hitcomponent (Collision|BreakHitResult HitResult))
  (bind (_bblockinghit_2 _binitialoverlap_2 _time_2 _distance_2 _location_2 _impactpoint_2 _normal_2 _impactnormal_2 _physmat_2 _hitactor_2) (Collision|BreakHitResult HitResult))
  (Utilities|FlowControl|Sequence
    (:then_0
      ;[1 1 1] Apply Damage
      (Game|Damage|ApplyPointDamage _hitactor_2 (Variables|Default|GetWeaponDamageValue) _normal_2 HitResult (Pawn|GetController (Variables|Default|GetOwningCharacter)) self (Variables|Default|GetWeaponDamageType)))
    (:then_1
      ;[1 1 1] Apply Impulse
      (Utilities|IsValid _hitcomponent
        (:Is%20Valid
          (if (Physics|IsSimulatingPhysics _hitcomponent "None")
            (CallFunction|AttackImpulse _hitcomponent)))))
    (:then_2
      ;[1 1 1] Impact Effects
      (Niagara|SpawnSystematLocation (Variables|Default|GetWeaponImpactEffect) _impactpoint)
      (bind _aspick_up_object (Utilities|Casting|CastToPickUpObject _hitactor)
        (:then
          (Audio|PlaySoundatLocation (Variables|/Game/Core/Blueprints/PickUpObject.PickUpObject_C|GetHitSound _aspick_up_object) _location "0, 0, 0" 1.0 1.0 0.0 0 0 0 0))
        (:CastFailed
          (Audio|PlaySoundatLocation (Variables|Default|GetWeaponImpactSound) _location "0, 0, 0" 1.0 1.0 0.0 0 0 0 0))))
    (:then_3
      (CallFunction|HitEffect HitResult))))

(fn GetAttackOrigin
  (bind _owningcharacter (Variables|Default|GetOwningCharacter))
  (return (+ (Transformation|GetActorLocation _owningcharacter) (* (Transformation|GetActorForwardVector _owningcharacter) (Variables|Default|GetAttackRange)))))

(fn AttackImpulse
  (params (HitComponent :type Primitive%20Component%20Object%20Reference))
  (Physics|AddImpulse HitComponent (+ (* (Transformation|GetActorForwardVector (Variables|Default|GetOwningCharacter)) (Variables|Default|GetAttackImpulseStrength)) "0, 0,100.000000") "None" true))