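; Ranged weapon Blueprint that fires a damaging laser beam from its AttackEffect event.
; A camera trace finds the aim point, then a second trace from the fire point finds the impact, though the start updates only when the camera trace hits.
; A Niagara beam spans the points and the hit actor takes damage.
; Secondary-fire and animation-end events are empty, leaving aim-camera timeline and repeat-attack logic disconnected.
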(event EventSecondaryStarted
  ;[1 1 1] Animations
)

(event EventSecondaryEnded
  ;[1 1 1] Animations
)

(event EventAttackEffect
  (bind _owningcharacter (Variables|Default|GetOwningCharacter))
  (bind _followcamera (Variables|/Game/Framework/Blueprints/PlayerCharacter.PlayerCharacter_C|GetFollowCamera _owningcharacter))
  (bind _returnvalue (Transformation|GetWorldLocation _followcamera))
  ;[1 1 1] Line Trace
  (bind (_outhit _returnvalue_2) (Collision|LineTraceByChannel _returnvalue (+ _returnvalue (* (Math|Vector|GetForwardVector _followcamera) 2e+03)) "TraceTypeQuery1" false 0 "None"))
  (if _returnvalue_2
    (Variables|Default|SetEndLoc (.Location (Collision|BreakHitResult _outhit)))
    (bind _output_get (Variables|Default|SetStartLoc (Transformation|GetWorldLocation (Variables|Default|GetFirePoint))))
    (else
      (Variables|Default|SetEndLoc (.TraceEnd (Collision|BreakHitResult _outhit)))))
  (bind (_outhit_2 _returnvalue_3) (Collision|LineTraceByChannel _output_get (Variables|Default|GetEndLoc) "TraceTypeQuery1" false 0 "None"))
  (if _returnvalue_3
    (Variables|Default|SetEndLoc (.Location (Collision|BreakHitResult _outhit_2))))
  (bind _returnvalue_4 (Niagara|SpawnSystematLocation "/Game/StudentWork/Particles/NS_LaserBeam.NS_LaserBeam" "0, 0, 0"))
  (Niagara|SetNiagaraVariable(Vector3) _returnvalue_4 "BeamStart" (Variables|Default|GetStartLoc))
  (Niagara|SetNiagaraVariable(Vector3) _returnvalue_4 "BeamEnd" (Variables|Default|GetEndLoc))
  (Niagara|SetNiagaraVariable(Vector3) _returnvalue_4 "ExplosiveOffset" (- (Variables|Default|GetStartLoc) (Variables|Default|GetEndLoc)))
  (Game|Damage|ApplyDamage (.HitActor (Collision|BreakHitResult _outhit_2)) 5.0 0 0))

(event EventFinishAttackAnim
  ;[1 1 1] Animations
)

(fn ConstructionScript
  (|CallParentFunction))