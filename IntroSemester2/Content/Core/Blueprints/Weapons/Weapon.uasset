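; Base weapon actor that characters pick up through their WeaponManager, drop as a physics object and attack with.
; Attack plays combo montages in sequence, repeating on blend-out until EndAttack, with a timer set for combo reset.
; Montage notifies call AttackEffect, an empty hook like draw, holster and secondary action, apparently for child weapons.
; Saves ownership state and transform, restoring the transform on load only when unowned.
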(event Custom|Reset%20Attack%20Combo
  (Variables|Default|SetAttackComboAnimCount 0))

(event Custom|HolsterWeapon)

(event Custom|SecondaryEnded)

(event Custom|DropWeapon
  (bind _box (Variables|Default|GetBox))
  (Variables|Default|SetOwningCharacter 0)
  (Collision|SetCollisionEnabled _box "QueryAndPhysics")
  (Physics|SetSimulatePhysics _box true))

(event Custom|IncreaseCombo
  (bind _result (Math|Integer|IncrementInt (Variables|Default|GetAttackComboAnimCount))
    (:%20%20
      (if (> _result (CallFunction|GetMaxCombo))
        (Variables|Default|SetAttackComboAnimCount 0))
      (Utilities|Time|SetTimerbyEvent (EventDispatchers|CreateEvent :!event Custom|Reset%20Attack%20Combo) 1.0))))

(event Custom|Finish%20Attack%20Anim
  (if (Variables|Default|GetRepeatAttack)
    (CallFunction|Attack)))

(event Custom|Attack
  (Variables|Default|SetRepeatAttack true)
  (if (not (Animation|Montage|MontageIsPlaying (Components|SkeletalMesh|GetAnimInstance (Variables|/Script/Engine.Character|GetMesh (Variables|Default|GetOwningCharacter))) 0))
    (Animation|Montage|PlayMontage (Variables|/Script/Engine.Character|GetMesh (Variables|Default|GetOwningCharacter)) (Utilities|Array|Get(acopy) (Variables|Animation|GetWeaponAttackAnims) (Variables|Default|GetAttackComboAnimCount)) 2.0
      (:then
        (CallFunction|IncreaseCombo))
      (:OnBlendOut
        (CallFunction|FinishAttackAnim))
      (:OnNotifyBegin
        (CallFunction|AttackEffect)))))

(event Custom|InitWeapon
  (params (Character :type Player%20Character%20Object%20Reference))
  (bind _box (Variables|Default|GetBox))
  (Variables|Default|SetOwningCharacter Character)
  (Physics|SetSimulatePhysics _box false)
  (Collision|SetCollisionEnabled _box "NoCollision"))

(event Custom|DrawWeapon)

(event Custom|SecondaryAction
  (params (isPressed :type Boolean))
  (if isPressed
    (CallFunction|SecondaryStarted)
    (else
      (CallFunction|SecondaryEnded))))

(event Custom|EndAttack
  (Variables|Default|SetRepeatAttack false))

(event Custom|AttackEffect)

(event Custom|SecondaryStarted)

(event EventInteract
  (params (Player :type Player%20Character%20Object%20Reference))
  (Utilities|IsValid (Variables|Default|GetOwningCharacter)
    (:Is%20Not%20Valid
      (Default|AddWeapon (Variables|/Game/Framework/Blueprints/PlayerCharacter.PlayerCharacter_C|GetWeaponManager Player) self))))

(event EventLoadData
  (params (ActorState :type Boolean) (ActorData :type Transform))
  (if (not ActorState)
    (Transformation|SetActorTransform ActorData)))

(fn ConstructionScript)

(fn GetMaxCombo
  (return (- (Utilities|Array|Length (Variables|Animation|GetWeaponAttackAnims)) 1)))

(fn SaveData
  (return (Utilities|IsValid (Variables|Default|GetOwningCharacter)) (Transformation|GetActorTransform)))