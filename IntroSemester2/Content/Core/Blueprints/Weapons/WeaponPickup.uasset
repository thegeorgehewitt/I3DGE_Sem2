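; Weapon pickup Blueprint that displays a configurable weapon class through a child actor, set in the construction script.
; On BeginPlay a timeline bobs the child actor up and down while rotating it around yaw.
; Interact only stores the class of the player's current weapon in a temporary variable; the nodes to add a weapon and swap the displayed class are disconnected.
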(event EventInteract
  (params (Player :type Player%20Character%20Object%20Reference))
  (Variables|Default|SetTempWeapon (Utilities|GetClass (Variables|/Game/Core/Blueprints/Components/BP_WeaponManager.BP_WeaponManager_C|GetCurrentWeapon (Variables|/Game/Framework/Blueprints/PlayerCharacter.PlayerCharacter_C|GetWeaponManager Player)))))

(event EventBeginPlay
  (bind (_direction _movementalpha _rotalpha) (Timeline|T_Bob Play)
    (:Update
      (Transformation|SetRelativeLocationAndRotation (Variables|Default|GetWeaponChild) (Math|Vector|Lerp(Vector) "0, 0,50.000000" "0.000000,0.000000,100.000000" _movementalpha) (Math|Rotator|Lerp(Rotator) "0, 0, 0" "0,360.000000, 0" _rotalpha) false false))))

(fn ConstructionScript
  (ChildActorComponent|SetChildActorClass (Variables|Default|GetWeaponChild) (Variables|Default|GetWeaponClass)))