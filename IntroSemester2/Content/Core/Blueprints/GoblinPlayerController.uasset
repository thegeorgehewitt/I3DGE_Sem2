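; Player controller that captures the goblin game's movement, look, jump and action inputs and forwards them to the controlled pawn.
; Each input becomes a message call on the pawn, with buttons sending true on press and false on release.
; Movement directions come from control rotation yaw only, keeping motion on the plane.
; Turn and look rate axes are scaled by a base rate and frame delta time.
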(event Input|ActionEvents|InputActionPrimaryAction
  (params (Key :type Key%20Structure :default "None"))
  (bind _returnvalue (Pawn|GetControlledPawn))
  (:Pressed
    (Class|InputInterface|PrimaryAction(Message) _returnvalue true))
  (:Released
    (Class|InputInterface|PrimaryAction(Message) _returnvalue false)))

(event Input|ActionEvents|InputActionSecondaryAction
  (params (Key :type Key%20Structure :default "None"))
  (bind _returnvalue (Pawn|GetControlledPawn))
  (:Pressed
    (Class|InputInterface|SecondaryAction(Message) _returnvalue true))
  (:Released
    (Class|InputInterface|SecondaryAction(Message) _returnvalue false)))

(event Input|ActionEvents|InputActionInteractAction
  (params (Key :type Key%20Structure :default "None"))
  (bind _returnvalue (Pawn|GetControlledPawn))
  (:Pressed
    (Class|InputInterface|InteractAction(Message) _returnvalue true))
  (:Released
    (Class|InputInterface|InteractAction(Message) _returnvalue false)))

(event Input|ActionEvents|InputActionJump
  (params (Key :type Key%20Structure :default "None"))
  (bind _returnvalue (Pawn|GetControlledPawn))
  (:Pressed
    (Class|InputInterface|JumpInput(Message) _returnvalue true))
  (:Released
    (Class|InputInterface|JumpInput(Message) _returnvalue false)))

(event Input|AxisEvents|InputAxisLookUp
  (params (AxisValue :type Float%20%28single-precision%29))
  (Class|InputInterface|LookUpInput(Message) (Pawn|GetControlledPawn) AxisValue))

(event Input|AxisEvents|InputAxisTurnRate
  (params (AxisValue :type Float%20%28single-precision%29))
  (Class|InputInterface|TurnInput(Message) (Pawn|GetControlledPawn) (* AxisValue (Variables|Default|GetBaseTurnRate) (Utilities|Time|GetWorldDeltaSeconds))))

(event Input|AxisEvents|InputAxisTurn
  (params (AxisValue :type Float%20%28single-precision%29))
  (Class|InputInterface|TurnInput(Message) (Pawn|GetControlledPawn) AxisValue))

(event Input|AxisEvents|InputAxisLookUpRate
  (params (AxisValue :type Float%20%28single-precision%29))
  (Class|InputInterface|LookUpInput(Message) (Pawn|GetControlledPawn) (* AxisValue (Variables|Default|GetBaseTurnRate) (Utilities|Time|GetWorldDeltaSeconds))))

(event Input|AxisEvents|InputAxisMoveForward
  (params (AxisValue :type Float%20%28single-precision%29))
  (Class|InputInterface|MoveForwardInput(Message) (Pawn|GetControlledPawn) (Math|Vector|GetForwardVector (Math|Rotator|MakeRotator 0.0 0.0 (.Yaw (Math|Rotator|BreakRotator (Pawn|GetControlRotation :!class /Script/Engine.Controller))))) AxisValue))

(event Input|AxisEvents|InputAxisMoveRight
  (params (AxisValue :type Float%20%28single-precision%29))
  (Class|InputInterface|MoveRightInput(Message) (Pawn|GetControlledPawn) (Math|Vector|GetRightVector (Math|Rotator|MakeRotator 0.0 0.0 (.Yaw (Math|Rotator|BreakRotator (Pawn|GetControlRotation :!class /Script/Engine.Controller))))) AxisValue))

(fn ConstructionScript)