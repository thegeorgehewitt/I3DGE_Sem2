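; BP_LevelEnd is a level exit actor with a gate mesh and a box trigger.
; When a PlayerCharacter overlaps the box, it calls FinishLevel on that character, with no check on whether the gate is unlocked.
; The Unlock event plays a timeline that lerps the gate downward from its starting relative location, then destroys the gate component when finished.
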(event OnComponentBeginOverlap(Box)
  (params (OverlappedComponent :type Primitive%20Component%20Object%20Reference) (OtherActor :type Actor%20Object%20Reference) (OtherComp :type Primitive%20Component%20Object%20Reference) (OtherBodyIndex :type Integer) (bFromSweep :type Boolean) (SweepResult :type Hit%20Result%20Structure%20%28by%20ref%29))
  (bind _asplayer_character (Utilities|Casting|CastToPlayerCharacter OtherActor))
  (Default|FinishLevel _asplayer_character))

(event Custom|Unlock
  (Variables|Default|SetGateStart (Variables|/Script/Engine.SceneComponent|GetRelativeLocation (Variables|Default|GetSM_Gate)))
  (bind _alpha (Timeline|GateMovement Play)
    (:Update
      (Transformation|SetRelativeLocation (Variables|Default|GetSM_Gate) (Math|Vector|Lerp(Vector) (Variables|Default|GetGateStart) (Math|Vector|MakeVector (.X (Class|KismetMathLibrary|BreakVector3f (Variables|Default|GetGateStart))) (.Y (Class|KismetMathLibrary|BreakVector3f (Variables|Default|GetGateStart))) (- (.Z (Class|KismetMathLibrary|BreakVector3f (Variables|Default|GetGateStart))) 58.0)) _alpha) false false))
    (:Finished
      (Components|DestroyComponent (Variables|Default|GetSM_Gate)))))

(event EventBeginPlay)

(event Collision|EventActorBeginOverlap
  (params (OtherActor :type Actor%20Object%20Reference)))

(event EventTick
  (params (DeltaSeconds :type Float%20%28single-precision%29)))

(fn ConstructionScript)