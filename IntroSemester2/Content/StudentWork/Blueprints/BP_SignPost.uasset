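; BP_SignPost is a signpost that shows a text widget while something is within its trigger sphere.
; On BeginPlay it passes TextToShow to its WBP_SignPost widget, then hides the widget component.
; Sphere overlap begin and end events toggle the widget's visibility, with no check on which actor or component overlaps.
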(event OnComponentBeginOverlap(Sphere)
  (params (OverlappedComponent :type Primitive%20Component%20Object%20Reference) (OtherActor :type Actor%20Object%20Reference) (OtherComp :type Primitive%20Component%20Object%20Reference) (OtherBodyIndex :type Integer) (bFromSweep :type Boolean) (SweepResult :type Hit%20Result%20Structure%20%28by%20ref%29))
  (Rendering|SetVisibility (Variables|Default|GetWidget) true false))

(event OnComponentEndOverlap(Sphere)
  (params (OverlappedComponent :type Primitive%20Component%20Object%20Reference) (OtherActor :type Actor%20Object%20Reference) (OtherComp :type Primitive%20Component%20Object%20Reference) (OtherBodyIndex :type Integer))
  (Rendering|SetVisibility (Variables|Default|GetWidget) false false))

(event EventBeginPlay
  (bind _aswbp_sign_post (Utilities|Casting|CastToWBP_SignPost (UserInterface|GetUserWidgetObject (Variables|Default|GetWidget))))
  (Default|UpdateSignPost _aswbp_sign_post (Variables|Default|GetText%20to%20Show))
  (Rendering|SetVisibility (Variables|Default|GetWidget) false false))

(fn ConstructionScript)