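; BP_GoalHoop is a scoring hoop that counts VictoryBall hits and unlocks the level end once a target score is reached.
; Its Box component's begin overlap filters for VictoryBall, increments Score and prints it to screen.
; When Score meets or exceeds TargetScore, it prints a message and calls Unlock on the LevelEnd reference, repeating on any later scoring overlap.
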(event OnComponentBeginOverlap(Box)
  (params (OverlappedComponent :type Primitive%20Component%20Object%20Reference) (OtherActor :type Actor%20Object%20Reference) (OtherComp :type Primitive%20Component%20Object%20Reference) (OtherBodyIndex :type Integer) (bFromSweep :type Boolean) (SweepResult :type Hit%20Result%20Structure%20%28by%20ref%29))
  (bind _score (Variables|Default|GetScore))
  (Utilities|Casting|CastToVictoryBall OtherActor)
  (Development|PrintString "Score!")
  (Math|Integer|IncrementInt _score
    (:%20%20
      (Development|PrintString (Utilities|String|ToString(Integer) _score))
      (if (>= (Variables|Default|GetScore) (Variables|Default|GetTargetScore))
        (Development|PrintString "Target Score Reached!")
        (Default|Unlock (Variables|Default|GetLevelEnd))))))

(event EventBeginPlay)

(event Collision|EventActorBeginOverlap
  (params (OtherActor :type Actor%20Object%20Reference)))

(event EventTick
  (params (DeltaSeconds :type Float%20%28single-precision%29)))

(fn ConstructionScript)