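; Target dummy actor that takes damage and explodes when destroyed.
; On BeginPlay it fills Health from MaxHealth, and each AnyDamage event subtracts the incoming damage.
; When Health reaches zero or below, it spawns a vertically stretched plasma explosion effect at its location and destroys itself.
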(event EventBeginPlay
  (Variables|Default|SetHealth (Variables|Default|GetMaxHealth)))

(event Game|Damage|EventAnyDamage
  (params (Damage :type Float%20%28single-precision%29) (DamageType :type Damage%20Type%20Object%20Reference) (InstigatedBy :type Controller%20Object%20Reference) (DamageCauser :type Actor%20Object%20Reference))
  (bind _output_get (Variables|Default|SetHealth (- (Variables|Default|GetHealth) Damage)))
  (if (<= _output_get 0.0)
    (Niagara|SpawnSystematLocation "/Game/Core/Particles/Niagara/PS_PlasmaExplode.PS_PlasmaExplode" (Transformation|GetActorLocation) "0, 0, 0" "1.000000,1.000000,3.000000")
    (Actor|DestroyActor)))

(fn ConstructionScript)