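; Crate puzzle door that swings open once it has received enough solutions.
; SolutionReceived and SolutionRemoved adjust a counter, which is kept from dropping below zero.
; Reaching SolutionsNeeded plays the OpenDoor timeline, lerping the root from its starting rotation through a 90-degree turn.
; Removing a solution only lowers the count and never closes the door.
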(event Custom|SolutionReceived
  (bind _startrotation (Variables|Default|GetStartRotation))
  (if (< (Variables|Default|GetSolutionsReceived) (Variables|Default|GetSolutionsNeeded))
    (bind _result (Math|Integer|IncrementInt (Variables|Default|GetSolutionsReceived))
      (:%20%20
        (if (>= _result (Variables|Default|GetSolutionsNeeded))
          (bind _alpha (Timeline|OpenDoor Play)
            (:Update
              (Transformation|SetWorldRotation (Variables|Default|GetDefaultSceneRoot) (Math|Rotator|Lerp(Rotator) _startrotation (Math|Rotator|CombineRotators _startrotation "0.000000,90.000000,0.000000") _alpha) false false))))))))

(event Custom|SolutionRemoved
  (bind _result (Math|Integer|DecrementInt (Variables|Default|GetSolutionsReceived))
    (:%20%20
      (if (< _result 0)
        (Variables|Default|SetSolutionsReceived 0)))))

(event EventBeginPlay
  (Variables|Default|SetSolutionsReceived 0)
  (Variables|Default|SetStartRotation (Transformation|GetWorldRotation (Variables|Default|GetDefaultSceneRoot))))

(fn ConstructionScript)