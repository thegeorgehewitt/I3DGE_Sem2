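; BP_SolutionTorch is a torch actor in the crates puzzle folder, with a flickering point light and a Niagara effect.
; On BeginPlay it zeroes the light, activates the effect and starts a looping timer that randomizes the light intensity ten times a second.
; The collision overlap events are empty, and leftover intensity logic is never run, so the torch does not react to overlaps.
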(event OnComponentBeginOverlap(Collision)
  (params (OverlappedComponent :type Primitive%20Component%20Object%20Reference) (OtherActor :type Actor%20Object%20Reference) (OtherComp :type Primitive%20Component%20Object%20Reference) (OtherBodyIndex :type Integer) (bFromSweep :type Boolean) (SweepResult :type Hit%20Result%20Structure%20%28by%20ref%29)))

(event OnComponentEndOverlap(Collision)
  (params (OverlappedComponent :type Primitive%20Component%20Object%20Reference) (OtherActor :type Actor%20Object%20Reference) (OtherComp :type Primitive%20Component%20Object%20Reference) (OtherBodyIndex :type Integer)))

(event Custom|Flicker
  (Rendering|Components|Light|SetIntensity (Variables|Default|GetPointLight) (Math|Random|RandomFloatinRange 5e+03 9e+03)))

(event EventBeginPlay
  (Rendering|Components|Light|SetIntensity (Variables|Default|GetPointLight) 0.0)
  (Components|Activation|Activate (Variables|Default|GetNiagara) false)
  (Utilities|Time|SetTimerbyEvent (delegate Custom|Flicker) 0.1 true))

(fn ConstructionScript)