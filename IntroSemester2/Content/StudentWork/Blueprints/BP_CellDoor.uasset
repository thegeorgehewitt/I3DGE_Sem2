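; BP_CellDoor is a cell door that toggles open and closed when it takes damage instigated by a player controller.
; It stores the mesh's world rotation at BeginPlay as the closed pose.
; A Timeline alpha lerps the mesh to a fixed angular offset from that pose, playing forward to open and reversing from the end to close.
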(event EventBeginPlay
  (Variables|Default|SetStartRotation (Transformation|GetWorldRotation (Variables|Default|GetStaticMesh))))

(event Game|Damage|EventAnyDamage
  (params (Damage :type Float%20%28single-precision%29) (DamageType :type Damage%20Type%20Object%20Reference) (InstigatedBy :type Controller%20Object%20Reference) (DamageCauser :type Actor%20Object%20Reference))
  (bind _startrotation (Variables|Default|GetStartRotation))
  (Utilities|Casting|CastToPlayerController InstigatedBy)
  (if (Variables|Default|GetOpen)
    (Variables|Default|SetOpen false)
    (bind _alpha (Timeline|Timeline ReverseFromEnd)
      (:Update
        (Transformation|SetWorldRotation (Variables|Default|GetStaticMesh) (Math|Rotator|Lerp(Rotator) _startrotation (Math|Rotator|CombineRotators _startrotation "0.000000,-65.000000,0.000000") _alpha true) false false)))
    (else
      (Variables|Default|SetOpen true)
      (Timeline|Timeline Play))))

(fn ConstructionScript)