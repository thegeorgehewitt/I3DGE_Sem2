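; Door that opens when the player solves a lock widget shown while standing in its trigger box.
; On BeginPlay it creates WBP_Lock, passing itself and its Solution values.
; Box overlaps toggle the widget, mouse cursor and look input until solved.
; SolutionRecieved and SolutionRemoved update three flags; when all are true, it closes the UI and swings the door 90 degrees via a delayed timeline.
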(event OnComponentBeginOverlap(Box)
  (params (OverlappedComponent :type Primitive%20Component%20Object%20Reference) (OtherActor :type Actor%20Object%20Reference) (OtherComp :type Primitive%20Component%20Object%20Reference) (OtherBodyIndex :type Integer) (bFromSweep :type Boolean) (SweepResult :type Hit%20Result%20Structure%20%28by%20ref%29))
  (bind _returnvalue (Game|GetPlayerController 0))
  (if (not (Variables|Default|GetSolved))
    (UserInterface|Viewport|AddtoViewport (Variables|Default|GetWidget) 0)
    (Variables|/Script/Engine.PlayerController|SetbShowMouseCursor _returnvalue true)
    (Input|SetIgnoreLookInput _returnvalue true)))

(event OnComponentEndOverlap(Box)
  (params (OverlappedComponent :type Primitive%20Component%20Object%20Reference) (OtherActor :type Actor%20Object%20Reference) (OtherComp :type Primitive%20Component%20Object%20Reference) (OtherBodyIndex :type Integer))
  (bind _returnvalue (Game|GetPlayerController 0))
  (if (not (Variables|Default|GetSolved))
    (Widget|RemovefromParent (Variables|Default|GetWidget))
    (Variables|/Script/Engine.PlayerController|SetbShowMouseCursor _returnvalue false)
    (Input|SetIgnoreLookInput _returnvalue false)))

(event Custom|OpenDoor
  (bind _returnvalue (Game|GetPlayerController 0))
  (bind _startrotation (Variables|Default|GetStartRotation))
  (Widget|RemovefromParent (Variables|Default|GetWidget))
  (Variables|/Script/Engine.PlayerController|SetbShowMouseCursor _returnvalue false)
  (Input|SetIgnoreLookInput _returnvalue false)
  (Input|SetInputModeGameOnly _returnvalue false)
  (Utilities|FlowControl|Delay 0.5)
  (bind _alpha (Timeline|Timeline Play)
    (:Update
      (Transformation|SetWorldRotation (Variables|Default|GetDoor) (Math|Rotator|Lerp(Rotator) _startrotation (Math|Rotator|CombineRotators _startrotation "0.000000,90.000000,0.000000") _alpha) false false))))

(event Custom|SolutionRecieved
  (params (Index :type Integer))
  (Utilities|Array|SetArrayElem (Variables|Default|GetSolve) Index true)
  (if (Math|Boolean|ANDBoolean (Utilities|Array|Get(acopy) (Variables|Default|GetSolve)) (Utilities|Array|Get(acopy) (Variables|Default|GetSolve) 1) (Utilities|Array|Get(acopy) (Variables|Default|GetSolve) 2))
    (Variables|Default|SetSolved true)
    (CallFunction|OpenDoor)))

(event Custom|SolutionRemoved
  (params (Index :type Integer))
  (Utilities|Array|SetArrayElem (Variables|Default|GetSolve) Index false))

(event EventBeginPlay
  (bind _returnvalue (UserInterface|CreateWidget "/Game/StudentWork/UI/WBP_Lock.WBP_Lock_C"))
  (bind _output_get (Variables|Default|SetWidget _returnvalue))
  (Variables|/Game/StudentWork/UI/WBP_Lock.WBP_Lock_C|SetDoor _output_get self)
  (for (_ _array_index) (Variables|/Game/StudentWork/UI/WBP_Lock.WBP_Lock_C|GetSolution _output_get)
    (Utilities|Array|SetArrayElem (Variables|/Game/StudentWork/UI/WBP_Lock.WBP_Lock_C|GetSolution _output_get) _array_index (Utilities|Array|Get(acopy) (Variables|Default|GetSolution) _array_index))
    (Variables|Default|SetStartRotation (Transformation|GetWorldRotation (Variables|Default|GetDoor)))))

(fn ConstructionScript)