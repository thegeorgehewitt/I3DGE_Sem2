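; BP_LightSequence is a trigger actor that lights a set of braziers and a spotlight when the player enters its collision volume.
; On BeginPlay it turns off each brazier's Niagara effect and point light and zeroes the spotlight's intensity.
; On overlap by PlayerCharacter it calls FadeIn on every brazier, spawns a dust Niagara effect at an arrow component, and ramps the spotlight toward IntensityGoal with a timeline.
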(event OnComponentBeginOverlap(Collision)
  (params (OverlappedComponent :type Primitive%20Component%20Object%20Reference) (OtherActor :type Actor%20Object%20Reference) (OtherComp :type Primitive%20Component%20Object%20Reference) (OtherBodyIndex :type Integer) (bFromSweep :type Boolean) (SweepResult :type Hit%20Result%20Structure%20%28by%20ref%29))
  (bind _arrow (Variables|Default|GetArrow))
  (bind _returnvalue (Transformation|GetWorldTransform _arrow))
  (Utilities|Casting|CastToPlayerCharacter OtherActor)
  (for _array_element (Variables|Default|GetBrazierLights)
    (Default|Fadein _array_element))
  (Niagara|SpawnSystematLocation "/Game/StudentWork/Particles/NS_Dust.NS_Dust" (.location _returnvalue) (.rotation _returnvalue))
  (bind _newtrack_0 (Timeline|Timeline Play)
    (:Update
      (Rendering|Components|Light|SetIntensity (Variables|/Script/Engine.Light|GetLightComponent (Variables|Default|GetSpotLight)) (* _newtrack_0 (Variables|Default|GetIntensityGoal))))))

(event EventBeginPlay
  (for _array_element (Variables|Default|GetBrazierLights)
    (Components|Activation|SetActive (Variables|/Game/StudentWork/Blueprints/LightAndFire/BP_FireForTorchNonFlicker.BP_FireForTorchNonFlicker_C|GetNiagara _array_element) false false)
    (Rendering|Components|Light|SetIntensity (Variables|/Game/StudentWork/Blueprints/LightAndFire/BP_FireForTorchNonFlicker.BP_FireForTorchNonFlicker_C|GetPointLight _array_element) 0.0)
    (Rendering|Components|Light|SetIntensity (Variables|/Script/Engine.Light|GetLightComponent (Variables|Default|GetSpotLight)) 0.0)))

(fn ConstructionScript)