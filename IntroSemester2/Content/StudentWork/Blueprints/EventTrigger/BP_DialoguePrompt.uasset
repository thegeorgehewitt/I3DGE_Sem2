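; BP_DialoguePrompt is a trigger actor that shows a dialogue prompt on screen while something overlaps its box.
; On BeginPlay it creates a WBP_HelperWidget once and fills it with its dialogue and speaker text variables.
; Box overlap begin adds the cached widget to the viewport and overlap end removes it, with no check on which actor overlaps.
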(event OnComponentBeginOverlap(Box)
  (params (OverlappedComponent :type Primitive%20Component%20Object%20Reference) (OtherActor :type Actor%20Object%20Reference) (OtherComp :type Primitive%20Component%20Object%20Reference) (OtherBodyIndex :type Integer) (bFromSweep :type Boolean) (SweepResult :type Hit%20Result%20Structure%20%28by%20ref%29))
  (UserInterface|Viewport|AddtoViewport (Variables|Default|GetHelper%20Widget) 0))

(event OnComponentEndOverlap(Box)
  (params (OverlappedComponent :type Primitive%20Component%20Object%20Reference) (OtherActor :type Actor%20Object%20Reference) (OtherComp :type Primitive%20Component%20Object%20Reference) (OtherBodyIndex :type Integer))
  (Widget|RemovefromParent (Variables|Default|GetHelper%20Widget)))

(event EventBeginPlay
  (bind _returnvalue (UserInterface|CreateWidget "/Game/StudentWork/UI/WBP_HelperWidget.WBP_HelperWidget_C"))
  (bind _output_get (Variables|Default|SetHelper%20Widget _returnvalue))
  (Default|UpdateDiaglogueText _output_get (Variables|Default|GetDialogueText) (Variables|Default|GetSpeakerText)))

(fn ConstructionScript)