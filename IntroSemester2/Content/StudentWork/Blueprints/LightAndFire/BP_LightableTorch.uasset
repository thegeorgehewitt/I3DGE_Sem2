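; BP_LightableTorch is a torch actor with a Niagara effect and flickering point light that gives color feedback on puzzle solutions.
; BeginPlay activates the effect and starts a looping timer that randomizes light intensity between MinIntensity and MaxIntensity.
; SolutionReceived and IncorrectSolutionReceived briefly tint the light green or red, then return it to warm orange.
; Collision overlap events are empty, and leftover intensity nodes never run.
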(event OnComponentBeginOverlap(Collision)
  (params (OverlappedComponent :type Primitive%20Component%20Object%20Reference) (OtherActor :type Actor%20Object%20Reference) (OtherComp :type Primitive%20Component%20Object%20Reference) (OtherBodyIndex :type Integer) (bFromSweep :type Boolean) (SweepResult :type Hit%20Result%20Structure%20%28by%20ref%29)))

(event OnComponentEndOverlap(Collision)
  (params (OverlappedComponent :type Primitive%20Component%20Object%20Reference) (OtherActor :type Actor%20Object%20Reference) (OtherComp :type Primitive%20Component%20Object%20Reference) (OtherBodyIndex :type Integer)))

(event Custom|Flicker
  (Rendering|Components|Light|SetIntensity (Variables|Default|GetPointLight) (Math|Random|RandomFloatinRange (Variables|Default|GetMinIntensity) (Variables|Default|GetMaxIntensity))))

(event Custom|SolutionReceived
  (Rendering|Components|Light|SetLightColor (Variables|Default|GetPointLight) "(R=0.271630,G=0.536458,B=0.225125,A=1.000000)" true)
  (Utilities|FlowControl|Delay 1.0)
  (Rendering|Components|Light|SetLightColor (Variables|Default|GetPointLight) "(R=1.000000,G=0.730461,B=0.371238,A=1.000000)" true))

(event Custom|IncorrectSolutionReceived
  (Rendering|Components|Light|SetLightColor (Variables|Default|GetPointLight) "(R=0.536458,G=0.111108,B=0.067057,A=1.000000)" true)
  (Utilities|FlowControl|Delay 1.0)
  (Rendering|Components|Light|SetLightColor (Variables|Default|GetPointLight) "(R=1.000000,G=0.730461,B=0.371238,A=1.000000)" true))

(event EventBeginPlay
  (Rendering|Components|Light|SetIntensity (Variables|Default|GetPointLight) 0.0)
  (Components|Activation|Activate (Variables|Default|GetNiagara) false)
  (bind _returnvalue (Utilities|Time|SetTimerbyEvent (delegate Custom|Flicker) 0.1 true))
  (Variables|Default|SetFlickerHandler _returnvalue))

(fn ConstructionScript)