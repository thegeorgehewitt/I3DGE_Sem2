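; BP_InsideLight is an interior light fixture that flickers continuously once play begins.
; A repeating three-second timer calls FlickeringStart, which sets or resets a looping one-second Flicker timer.
; Each flicker shows a blue emissive material at maximum intensity and radius, then after a half-second delay swaps materials and drops to minimum intensity.
; The dim phase feeds MaxIntensity into the attenuation radius.
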(event Custom|FlickeringStart
  (Utilities|Time|SetTimerbyEvent (delegate Custom|Flicker) 1.0 true))

(event Custom|Flicker
  (Rendering|Material|SetMaterial (Variables|Default|GetStaticMesh) 1 "/Game/Framework/DungeonKit/Materials/MI_EmissiveBlue.MI_EmissiveBlue")
  (Rendering|Components|Light|SetIntensity (Variables|Default|GetLight) (Variables|Default|GetMax%20Intensity))
  (Rendering|Lighting|SetAttenuationRadius (Variables|Default|GetLight) (Variables|Default|GetMax%20Atten%20Radius))
  (Utilities|FlowControl|Delay 0.5)
  (Rendering|Material|SetMaterial (Variables|Default|GetStaticMesh) 1 "/Game/Core/Animations/Alpha_Joints_MAT.Alpha_Joints_MAT")
  (Rendering|Components|Light|SetIntensity (Variables|Default|GetLight) (Variables|Default|GetMin%20Intensity))
  (Rendering|Lighting|SetAttenuationRadius (Variables|Default|GetLight) (Variables|Default|GetMax%20Intensity)))

(event EventBeginPlay
  (Rendering|Components|Light|SetIntensity (Variables|Default|GetLight) (Variables|Default|GetMax%20Intensity))
  (Rendering|Lighting|SetAttenuationRadius (Variables|Default|GetLight) (Variables|Default|GetMax%20Atten%20Radius))
  (Utilities|Time|SetTimerbyEvent (delegate Custom|FlickeringStart) 3.0 true))

(fn ConstructionScript)