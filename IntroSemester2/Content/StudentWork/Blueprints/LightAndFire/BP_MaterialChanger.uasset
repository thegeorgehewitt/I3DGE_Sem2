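; BP_MaterialChanger is an actor whose cube glows blue and flickers while a character stands inside its box collision.
; BeginPlay assigns an emissive blue material to one slot and creates a dynamic instance to drive its Glow parameter.
; Begin overlap from any Character starts a looping timer that randomizes Glow.
; End overlap clears the timer and restores the base glow, but only for PlayerCharacter.
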(event OnComponentBeginOverlap(BoxCollision)
  (params (OverlappedComponent :type Primitive%20Component%20Object%20Reference) (OtherActor :type Actor%20Object%20Reference) (OtherComp :type Primitive%20Component%20Object%20Reference) (OtherBodyIndex :type Integer) (bFromSweep :type Boolean) (SweepResult :type Hit%20Result%20Structure%20%28by%20ref%29))
  (Utilities|Casting|CastToCharacter OtherActor)
  (bind _returnvalue (Utilities|Time|SetTimerbyEvent (delegate Custom|Flicker) 0.2 true))
  (Variables|Default|SetFlickerTimer _returnvalue))

(event OnComponentEndOverlap(BoxCollision)
  (params (OverlappedComponent :type Primitive%20Component%20Object%20Reference) (OtherActor :type Actor%20Object%20Reference) (OtherComp :type Primitive%20Component%20Object%20Reference) (OtherBodyIndex :type Integer))
  (Utilities|Casting|CastToPlayerCharacter OtherActor)
  (Utilities|Time|ClearandInvalidateTimerbyHandle (Variables|Default|GetFlickerTimer))
  (Rendering|Material|SetScalarParameterValue (Variables|Default|GetMaterial) "Glow" 2.0 :!class /Script/Engine.MaterialInstanceDynamic))

(event Custom|Flicker
  (Rendering|Material|SetScalarParameterValue (Variables|Default|GetMaterial) "Glow" (Math|Random|RandomFloatinRange 1.0 4e+01) :!class /Script/Engine.MaterialInstanceDynamic))

(event EventBeginPlay
  (Rendering|Material|SetMaterial (Variables|Default|GetCubeMesh) 2 "/Game/Framework/DungeonKit/Materials/MI_EmissiveBlue.MI_EmissiveBlue")
  (bind _returnvalue (Rendering|Material|CreateDynamicMaterialInstance (Variables|Default|GetCubeMesh) 2 0 "None" :!class /Script/Engine.PrimitiveComponent))
  (Variables|Default|SetMaterial _returnvalue)
  (Rendering|Material|SetScalarParameterValue (Variables|Default|GetMaterial) "Glow" 2.0 :!class /Script/Engine.MaterialInstanceDynamic))

(fn ConstructionScript)