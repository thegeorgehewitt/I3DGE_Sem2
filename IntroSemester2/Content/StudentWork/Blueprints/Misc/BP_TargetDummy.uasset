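; BP_TargetDummy is a damageable barrel target with a health bar widget that explodes in a Niagara effect and destroys itself at zero health.
; A looping timer heals it through negative ApplyDamage, so hits and healing share the AnyDamage path that clamps health and updates the bar.
; Two health thresholds switch dynamic wood and metal materials between damage looks, though recovery never restores the wood colour because that parameter name is None.
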(event Custom|Heal
  (Game|Damage|ApplyDamage self -5.0 0 0))

(event EventBeginPlay
  (Variables|Default|SetHealth (Variables|Default|GetMaxHealth))
  (bind _returnvalue (Rendering|Material|CreateDynamicMaterialInstance (Variables|Default|GetStaticMesh) 0 0 "None" :!class /Script/Engine.PrimitiveComponent))
  (bind _output_get (Variables|Default|SetBarrelWoodMaterial _returnvalue))
  (bind _returnvalue_2 (Rendering|Material|GetScalarParameterValue _output_get "Roughness" :!class /Script/Engine.MaterialInstanceDynamic))
  (Variables|Default|SetDefaultRoughness _returnvalue_2)
  (bind _returnvalue_3 (Rendering|Material|GetVectorParameterValue _output_get "HueColourOverlay" :!class /Script/Engine.MaterialInstanceDynamic))
  (Variables|Default|SetDefaultColour _returnvalue_3)
  (bind _returnvalue_4 (Rendering|Material|CreateDynamicMaterialInstance (Variables|Default|GetStaticMesh) 1 0 "None" :!class /Script/Engine.PrimitiveComponent))
  (bind _output_get_2 (Variables|Default|SetBarrelMetalMaterial _returnvalue_4))
  (bind _returnvalue_5 (Rendering|Material|GetScalarParameterValue _output_get_2 "Metallic" :!class /Script/Engine.MaterialInstanceDynamic))
  (Variables|Default|SetDefaultMetallic _returnvalue_5)
  (bind _aswbp_health_bar (Utilities|Casting|CastToWBP_HealthBar (UserInterface|GetUserWidgetObject (Variables|Default|GetWidget))))
  (bind _output_get_3 (Variables|Default|SetAs%20WBP%20Health%20Bar _aswbp_health_bar))
  (Default|UpdateHPBar _output_get_3 self)
  (bind _returnvalue_6 (Utilities|Time|SetTimerbyEvent (delegate Custom|Heal) 5.0 true))
  (Variables|Default|SetTimerHandler _returnvalue_6))

(event Game|Damage|EventAnyDamage
  (params (Damage :type Float%20%28single-precision%29) (DamageType :type Damage%20Type%20Object%20Reference) (InstigatedBy :type Controller%20Object%20Reference) (DamageCauser :type Actor%20Object%20Reference))
  (Variables|Default|SetHealth (Math|Float|Clamp(Float) (- (Variables|Default|GetHealth) Damage) 0.0 (Variables|Default|GetMaxHealth)))
  (bind _aswbp_health_bar (Utilities|Casting|CastToWBP_HealthBar (UserInterface|GetUserWidgetObject (Variables|Default|GetWidget)))
    (:then
      (bind _output_get (Variables|Default|SetAs%20WBP%20Health%20Bar _aswbp_health_bar))
      (Default|UpdateHPBar _output_get self))
    (:CastFailed
      (Development|PrintString "cast failed")))
  (if (<= (Variables|Default|GetHealth) 0.0)
    (Niagara|SpawnSystematLocation "/Game/Core/Particles/Niagara/PS_PlasmaExplode.PS_PlasmaExplode" (Transformation|GetActorLocation) "0, 0, 0" "1.000000,1.000000,3.000000")
    (Utilities|Time|ClearandInvalidateTimerbyHandle (Variables|Default|GetTimerHandler))
    (Actor|DestroyActor)
    (else
      ;[1 1 1] Change Material
      (if (<= (/ (Variables|Default|GetHealth) (Variables|Default|GetMaxHealth)) 0.25)
        (Rendering|Material|SetScalarParameterValue (Variables|Default|GetBarrelWoodMaterial) "Roughness" (Variables|Default|GetDamage2Roughness) :!class /Script/Engine.MaterialInstanceDynamic)
        (Rendering|Material|SetVectorParameterValue (Variables|Default|GetBarrelWoodMaterial) "HueColourOverlay" (Variables|Default|GetDamage2Colour) :!class /Script/Engine.MaterialInstanceDynamic)
        (Rendering|Material|SetScalarParameterValue (Variables|Default|GetBarrelMetalMaterial) "Metallic" (Variables|Default|GetDamage2Metallic) :!class /Script/Engine.MaterialInstanceDynamic)
        (elif (<= (/ (Variables|Default|GetHealth) (Variables|Default|GetMaxHealth)) 0.6)
          (Rendering|Material|SetScalarParameterValue (Variables|Default|GetBarrelWoodMaterial) "Roughness" (Variables|Default|GetDamage1Roughness) :!class /Script/Engine.MaterialInstanceDynamic)
          (Rendering|Material|SetVectorParameterValue (Variables|Default|GetBarrelWoodMaterial) "HueColourOverlay" (Variables|Default|GetDamage1Colour) :!class /Script/Engine.MaterialInstanceDynamic)
          (Rendering|Material|SetScalarParameterValue (Variables|Default|GetBarrelMetalMaterial) "Metallic" (Variables|Default|GetDamage1Metallic) :!class /Script/Engine.MaterialInstanceDynamic)
          (else
            (Rendering|Material|SetScalarParameterValue (Variables|Default|GetBarrelWoodMaterial) "Roughness" (Variables|Default|GetDefaultRoughness) :!class /Script/Engine.MaterialInstanceDynamic)
            (Rendering|Material|SetVectorParameterValue (Variables|Default|GetBarrelWoodMaterial) "None" (Variables|Default|GetDefaultColour) :!class /Script/Engine.MaterialInstanceDynamic)
            (Rendering|Material|SetScalarParameterValue (Variables|Default|GetBarrelMetalMaterial) "Metallic" (Variables|Default|GetDefaultMetallic) :!class /Script/Engine.MaterialInstanceDynamic)))))))

(fn ConstructionScript)