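; BP_PlaqueRiddle is a plaque that shows riddle text on screen while the player character is near it.
; On BeginPlay it creates a WBP_RiddleText widget and fills it with its Riddle text.
; A sphere overlap adds the widget to the viewport when the PlayerCharacter enters and removes it when they leave.
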(event OnComponentBeginOverlap(Sphere)
  (params (OverlappedComponent :type Primitive%20Component%20Object%20Reference) (OtherActor :type Actor%20Object%20Reference) (OtherComp :type Primitive%20Component%20Object%20Reference) (OtherBodyIndex :type Integer) (bFromSweep :type Boolean) (SweepResult :type Hit%20Result%20Structure%20%28by%20ref%29))
  (Utilities|Casting|CastToPlayerCharacter OtherActor)
  (UserInterface|Viewport|AddtoViewport (Variables|Default|GetRiddleWidget) 0))

(event OnComponentEndOverlap(Sphere)
  (params (OverlappedComponent :type Primitive%20Component%20Object%20Reference) (OtherActor :type Actor%20Object%20Reference) (OtherComp :type Primitive%20Component%20Object%20Reference) (OtherBodyIndex :type Integer))
  (Utilities|Casting|CastToPlayerCharacter OtherActor)
  (Widget|RemovefromParent (Variables|Default|GetRiddleWidget)))

(event EventBeginPlay
  (bind _returnvalue (UserInterface|CreateWidget "/Game/StudentWork/UI/WBP_RiddleText.WBP_RiddleText_C"))
  (bind _output_get (Variables|Default|SetRiddleWidget _returnvalue))
  (Default|UpdateText _output_get (Variables|Default|GetRiddle)))

(fn ConstructionScript)