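; BP_ParameterChanger is an actor whose cube changes material appearance when something overlaps its box collision.
; BeginPlay creates a dynamic material instance on the cube mesh and stores it.
; Begin and end overlap switch the BaseColour and Roughness parameters between active and inactive values, with no filter on the overlapping actor.
; Both events set BaseTexture to the same StoneWall texture, so it does not revert on exit.
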(event OnComponentBeginOverlap(BoxCollision)
  (params (OverlappedComponent :type Primitive%20Component%20Object%20Reference) (OtherActor :type Actor%20Object%20Reference) (OtherComp :type Primitive%20Component%20Object%20Reference) (OtherBodyIndex :type Integer) (bFromSweep :type Boolean) (SweepResult :type Hit%20Result%20Structure%20%28by%20ref%29))
  (bind _defaultcubematerial (Variables|Default|GetDefaultCubeMaterial))
  (Rendering|Material|SetVectorParameterValue _defaultcubematerial "BaseColour" (Variables|Default|GetActiveColour) :!class /Script/Engine.MaterialInstanceDynamic)
  (Rendering|Material|SetScalarParameterValue _defaultcubematerial "Roughness" (Variables|Default|GetActiveRoughness) :!class /Script/Engine.MaterialInstanceDynamic)
  (Rendering|Material|SetTextureParameterValue _defaultcubematerial "BaseTexture" "/Game/Framework/DungeonKit/Textures/StoneWall.StoneWall"))

(event OnComponentEndOverlap(BoxCollision)
  (params (OverlappedComponent :type Primitive%20Component%20Object%20Reference) (OtherActor :type Actor%20Object%20Reference) (OtherComp :type Primitive%20Component%20Object%20Reference) (OtherBodyIndex :type Integer))
  (bind _defaultcubematerial (Variables|Default|GetDefaultCubeMaterial))
  (Rendering|Material|SetVectorParameterValue _defaultcubematerial "BaseColour" (Variables|Default|GetInactiveColour) :!class /Script/Engine.MaterialInstanceDynamic)
  (Rendering|Material|SetScalarParameterValue _defaultcubematerial "Roughness" (Variables|Default|GetInactiveRoughness) :!class /Script/Engine.MaterialInstanceDynamic)
  (Rendering|Material|SetTextureParameterValue _defaultcubematerial "BaseTexture" "/Game/Framework/DungeonKit/Textures/StoneWall.StoneWall"))

(event EventBeginPlay
  (bind _returnvalue (Rendering|Material|CreateDynamicMaterialInstance (Variables|Default|GetCubeMesh) 0 0 "None" :!class /Script/Engine.PrimitiveComponent))
  (Variables|Default|SetDefaultCubeMaterial _returnvalue))

(fn ConstructionScript)