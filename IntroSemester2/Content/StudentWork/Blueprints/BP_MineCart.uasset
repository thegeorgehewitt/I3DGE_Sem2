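; BP_MineCart is a puzzle mine cart with a rotatable tool, solved when cart position and tool rotation both match the solution.
; MoveCart starts or stops a timeline that drives the cart along a spline, flipping direction when a run finishes.
; Damage instigated by a player controller turns the tool 120 degrees, ignoring further hits until done.
; Both timelines update the Solved flag, checking a position range and a rotation tolerance.
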(event Custom|MoveCart
  (bind _splinepath (Variables|Default|GetSplinePath))
  (bind _spline (Variables|/Game/StudentWork/Blueprints/BP_CartSpline.BP_CartSpline_C|GetSpline _splinepath))
  (Components|Timeline|SetPlayRate (Variables|Default|GetCartMovement) (/ 1.0 (Variables|Default|GetTiemToMove)))
  (if (Variables|Default|GetMoving)
    (Variables|Default|SetMoving false)
    (bind _alpha (Timeline|CartMovement Stop)
      (:Update
        (bind _output_get (Variables|Default|SetLast%20Alpha _alpha))
        (Transformation|SetActorTransform (Math|Transform|MakeTransform (Spline|GetLocationatDistanceAlongSpline _spline (Math|Float|Lerp 0.0 (Spline|GetSplineLength (Variables|/Game/StudentWork/Blueprints/BP_CartSpline.BP_CartSpline_C|GetSpline (Variables|Default|GetSplinePath))) _alpha) "World") (Spline|GetRotationatDistanceAlongSpline _spline (Math|Float|Lerp 0.0 (Spline|GetSplineLength (Variables|/Game/StudentWork/Blueprints/BP_CartSpline.BP_CartSpline_C|GetSpline (Variables|Default|GetSplinePath))) _alpha) "Local") "1.000000,1.000000,1.000000"))
        (if (and (<= _output_get (Variables|Default|GetSolutionUpper)) (>= _output_get (Variables|Default|GetSolutionLower)))
          (Variables|Default|SetRange true)
          (if (Variables|Default|GetRotation)
            (Variables|Default|SetSolved true)
            (else
              (Variables|Default|SetSolved false :!label _label)))
          (else
            (Variables|Default|SetRange false)
            (goto _label))))
      (:Finished
        (Variables|Default|SetMoving false)
        (if (Variables|Default|GetForwards)
          (Variables|Default|SetForwards false)
          (else
            (Variables|Default|SetForwards true)))))
    (else
      (Variables|Default|SetMoving true)
      (if (Variables|Default|GetForwards)
        (Timeline|CartMovement Play)
        (else
          (Timeline|CartMovement Reverse))))))

(event Custom|RotateTool
  (Variables|Default|SetStartRotation (Transformation|GetWorldRotation (Variables|Default|GetTool)))
  (bind _newtrack_0 (Timeline|ToolRotation PlayFromStart)
    (:Update
      (Transformation|SetWorldRotation (Variables|Default|GetTool) (Math|Rotator|Lerp(Rotator) (Variables|Default|GetStartRotation) (Math|Rotator|CombineRotators (Variables|Default|GetStartRotation) "0.000000,0.000000,120.000000") _newtrack_0 true) false false)
      (bind _output_get (Variables|Default|SetRotation (Utilities|Operators|EqualEqual (Math|Rotator|Lerp(Rotator) (Variables|Default|GetStartRotation) (Math|Rotator|CombineRotators (Variables|Default|GetStartRotation) "0.000000,0.000000,120.000000") _newtrack_0 true) (Variables|Default|GetSolutionRotation) 5.0)))
      (if _output_get
        (if (Variables|Default|GetRange)
          (Variables|Default|SetSolved true)
          (else
            (Variables|Default|SetSolved false :!label _label)))
        (else
          (goto _label))))
    (:Finished
      (Variables|Default|SetIsHit false))))

(event Game|Damage|EventAnyDamage
  (params (Damage :type Float%20%28single-precision%29) (DamageType :type Damage%20Type%20Object%20Reference) (InstigatedBy :type Controller%20Object%20Reference) (DamageCauser :type Actor%20Object%20Reference))
  (Utilities|Casting|CastToPlayerController InstigatedBy)
  (if (not (Variables|Default|GetIsHit))
    (Variables|Default|SetIsHit true)
    (CallFunction|RotateTool)))

(fn ConstructionScript)