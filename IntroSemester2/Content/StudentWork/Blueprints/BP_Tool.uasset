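; BP_Tool is a tool actor that can be released from its owning character and attach itself to mine carts.
; A custom event clears the owner and turns on collision and physics simulation for its Box.
; When the Box begins overlapping a BP_MineCart while the player character is not the owner, the tool attaches to that cart with relative transforms.
; Its HitEffect event only prints a debug message on cart hits.
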(event OnComponentBeginOverlap(Box)
  (params (OverlappedComponent :type Primitive%20Component%20Object%20Reference) (OtherActor :type Actor%20Object%20Reference) (OtherComp :type Primitive%20Component%20Object%20Reference) (OtherBodyIndex :type Integer) (bFromSweep :type Boolean) (SweepResult :type Hit%20Result%20Structure%20%28by%20ref%29))
  (bind _asbp_mine_cart (Utilities|Casting|CastToBP_MineCart OtherActor))
  (if (not (== (Variables|Default|GetOwningCharacter) "/Game/Framework/Blueprints/PlayerCharacter.PlayerCharacter"))
    (Transformation|AttachActorToActor _asbp_mine_cart "None" "KeepRelative" "KeepRelative" "KeepRelative" true)))

(event Custom|CustomEvent
  (bind _box (Variables|Default|GetBox))
  (Variables|Default|SetOwningCharacter 0)
  (Collision|SetCollisionEnabled _box "QueryAndPhysics")
  (Physics|SetSimulatePhysics _box true))

(event EventHitEffect
  (params (AttackHit :type Hit%20Result%20Structure))
  (Utilities|Casting|CastToBP_MineCart (.hitactor AttackHit))
  (Development|PrintString "Hit Cart"))

(fn ConstructionScript
  (|CallParentFunction))