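; Lever switch in the shadow puzzle that moves a linked Cart when damaged by a player controller.
; Each accepted hit calls MoveCart on the Cart and toggles Forward, playing or reversing the RotateLever timeline to swing the lever mesh between its starting rotation and an offset.
; The IsHit guard clears right after MoveCart, so it only stays latched when the Cart is invalid.
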(event EventBeginPlay
  (Variables|Default|SetStartRotation (Transformation|GetWorldRotation (Variables|Default|GetStaticMesh1))))

(event Game|Damage|EventAnyDamage
  (params (Damage :type Float%20%28single-precision%29) (DamageType :type Damage%20Type%20Object%20Reference) (InstigatedBy :type Controller%20Object%20Reference) (DamageCauser :type Actor%20Object%20Reference))
  (bind _startrotation (Variables|Default|GetStartRotation))
  (Utilities|Casting|CastToPlayerController InstigatedBy)
  (if (not (Variables|Default|GetIsHit))
    (Variables|Default|SetIsHit true)
    (Utilities|IsValid (Variables|Default|GetCart)
      (:Is%20Valid
        (Default|MoveCart (Variables|Default|GetCart))
        (Variables|Default|SetIsHit false)
        (if (Variables|Default|GetForward)
          (Variables|Default|SetForward false)
          (bind _newtrack_0 (Timeline|RotateLever Play)
            (:Update
              (Transformation|SetWorldRotation (Variables|Default|GetStaticMesh1) (Math|Rotator|Lerp(Rotator) _startrotation (Math|Rotator|CombineRotators _startrotation "-60.000000,0.000000,0.000000") _newtrack_0 true) false false)))
          (else
            (Variables|Default|SetForward true)
            (Timeline|RotateLever Reverse)))))))

(fn ConstructionScript)