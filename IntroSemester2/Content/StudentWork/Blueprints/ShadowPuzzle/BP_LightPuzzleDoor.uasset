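; BP_LightPuzzleDoor is a shadow puzzle door that opens while both of its referenced carts report as solved.
; A looping timer started on BeginPlay polls both carts' Solved flags every half second.
; The OpenDoor timeline interpolates the root from its saved starting rotation through a 90-degree turn.
; It reverses whenever either cart is unsolved, so the door can close again.
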(event Custom|CheckSolutions
  (bind _startrotation (Variables|Default|GetStartRotation))
  (if (and (Variables|/Game/StudentWork/Blueprints/ShadowPuzzle/BP_MineCart.BP_MineCart_C|GetSolved (Variables|Default|GetCart1)) (Variables|/Game/StudentWork/Blueprints/ShadowPuzzle/BP_MineCart.BP_MineCart_C|GetSolved (Variables|Default|GetCart2)))
    (bind _alpha (Timeline|OpenDoor Play)
      (:Update
        (Transformation|SetWorldRotation (Variables|Default|GetDefaultSceneRoot) (Math|Rotator|Lerp(Rotator) _startrotation (Math|Rotator|CombineRotators _startrotation "0.000000,90.000000,0.000000") _alpha) false false)))
    (else
      (Timeline|OpenDoor Reverse))))

(event EventBeginPlay
  (Variables|Default|SetStartRotation (Transformation|GetWorldRotation (Variables|Default|GetDefaultSceneRoot)))
  (bind _returnvalue (Utilities|Time|SetTimerbyEvent (delegate Custom|CheckSolutions) 0.5 true))
  (Variables|Default|SetSolCheckHandler _returnvalue))

(fn ConstructionScript)