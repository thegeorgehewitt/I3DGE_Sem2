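; Puzzle detection zone that checks whether an overlapping PickUpBox is the correct answer for a linked Door.
; A box is correct when its second material matches the detector's mesh material and its first matches AnswerMat.
; Correct boxes notify the Door and optional LinkedTorch, while wrong boxes signal only the torch.
; Removing a correct box revokes the Door's solution but sends nothing to the torch.
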(event OnComponentBeginOverlap(Collision)
  (params (OverlappedComponent :type Primitive%20Component%20Object%20Reference) (OtherActor :type Actor%20Object%20Reference) (OtherComp :type Primitive%20Component%20Object%20Reference) (OtherBodyIndex :type Integer) (bFromSweep :type Boolean) (SweepResult :type Hit%20Result%20Structure%20%28by%20ref%29))
  (bind _linkedtorch (Variables|Default|GetLinkedTorch))
  (bind _linkedtorch_2 (Variables|Default|GetLinkedTorch))
  (bind _aspick_up_box (Utilities|Casting|CastToPickUpBox OtherActor))
  (if (== (Rendering|Material|GetMaterial (Variables|/Game/Core/Blueprints/PickUpObject.PickUpObject_C|GetStaticMesh _aspick_up_box) 1) (Rendering|Material|GetMaterial (Variables|Default|GetStaticMesh) 0))
    (if (== (Rendering|Material|GetMaterial (Variables|/Game/Core/Blueprints/PickUpObject.PickUpObject_C|GetStaticMesh _aspick_up_box) 0) (Variables|Default|GetAnswerMat))
      (Default|SolutionReceived (Variables|Default|GetDoor))
      (Utilities|IsValid _linkedtorch_2
        (:Is%20Valid
          (Default|SolutionReceived _linkedtorch_2)))
      (else
        (Utilities|IsValid _linkedtorch :!label _label
          (:Is%20Valid
            (Default|IncorrectSolutionReceived _linkedtorch)))))
    (else
      (goto _label))))

(event OnComponentEndOverlap(Collision)
  (params (OverlappedComponent :type Primitive%20Component%20Object%20Reference) (OtherActor :type Actor%20Object%20Reference) (OtherComp :type Primitive%20Component%20Object%20Reference) (OtherBodyIndex :type Integer))
  (bind _aspick_up_box (Utilities|Casting|CastToPickUpBox OtherActor))
  (if (== (Rendering|Material|GetMaterial (Variables|/Game/Core/Blueprints/PickUpObject.PickUpObject_C|GetStaticMesh _aspick_up_box) 1) (Rendering|Material|GetMaterial (Variables|Default|GetStaticMesh) 0))
    (if (== (Rendering|Material|GetMaterial (Variables|/Game/Core/Blueprints/PickUpObject.PickUpObject_C|GetStaticMesh _aspick_up_box) 0) (Variables|Default|GetAnswerMat))
      (Default|SolutionRemoved (Variables|Default|GetDoor)))))

(event EventBeginPlay)

(fn ConstructionScript)