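; BP_GlowingGrid is a Blueprint that animates a light to give a pulsing glow.
; On BeginPlay it plays a Timeline whose Pulsing track is remapped with clamping on every update to drive the light's intensity and attenuation radius together.
; Min and max variables set the range for each property, and the construction script is empty.
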(event EventBeginPlay
  (bind _pulsing (Timeline|Timeline Play)
    (:Update
      (Rendering|Components|Light|SetIntensity (Variables|Default|GetLight) (Math|Float|MapRangeClamped _pulsing 0.0 1.0 (Variables|Default|GetMinIntensity) (Variables|Default|GetMaxIntensity)))
      (Rendering|Lighting|SetAttenuationRadius (Variables|Default|GetLight) (Math|Float|MapRangeClamped _pulsing 0.0 1.0 (Variables|Default|GetMinAtten) (Variables|Default|GetMaxAtten))))))

(fn ConstructionScript)